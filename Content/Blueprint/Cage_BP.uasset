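; Cage of light tubes that lights up in patterns from music notes received over OSC, or from input actions.
; BeginPlay sets every tube to glass and binds OSC handlers, each matching the address to an instrument note such as kick, snare or vocals.
; Matches toggle tube groups (frames, crosses, horizontals, diagonals) through per-group Lit flags and On/Off material swaps.
; Most input actions light groups only while held, but LightSecondFrame toggles one back-cross tube.
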(event `InputAction|LightThirdFrame`
  (params (Key :type "Key Structure"))
  (:`Pressed`
    (`self.LightFrame` (`self.On`) 12 17 1 6))
  (:`Released`
    (`self.LightFrame` (`self.Off`) 12 17 1 6)))

(event `InputAction|LightSecondFrame`
  (params (Key :type "Key Structure"))
  (:`Pressed`
    (`self.Light Back Cross PArt 1`)))

(event `InputAction|LightFirstFrame`
  (params (Key :type "Key Structure"))
  (:`Pressed`
    (`self.LightFrame` (`self.On`) 11 8 0 21))
  (:`Released`
    (`self.LightFrame` (`self.Off`) 11 8 0 21)))

(event `InputAction|LightDiagonals`
  (params (Key :type "Key Structure"))
  (:`Pressed`
    (`self.LightFrame` (`self.On`) 13 3 2 14))
  (:`Released`
    (`self.LightFrame` (`self.Off`) 13 3 2 14)))

(event `InputAction|LightBackCross`
  (params (Key :type "Key Structure"))
  (:`Pressed`
    (`self.LightCross` (`self.On`) 20 9))
  (:`Released`
    (`self.LightCross` (`self.Off`) 20 9)))

(event `InputAction|LightFrontHorizontal`
  (params (Key :type "Key Structure"))
  (:`Pressed`
    (`self.LightHorizontal` (`self.On`) 11 23))
  (:`Released`
    (`self.LightHorizontal` (`self.Off`) 11 23)))

(event `InputAction|LightBackHorizontal`
  (params (Key :type "Key Structure"))
  (:`Pressed`
    (`self.LightHorizontal` (`self.On`) 12 9 1))
  (:`Released`
    (`self.LightHorizontal` (`self.Off`) 12 9 1)))

(event `InputAction|LightFrontCross`
  (params (Key :type "Key Structure"))
  (:`Pressed`
    (`self.LightCross` (`self.On`) 18 23))
  (:`Released`
    (`self.LightCross` (`self.Off`) 18 23)))

(event `self.ReceiveBeginPlay`
  (add `OscReceiverComponent.OnOscReceived` (`self.OscReceiver`) (delegate `OSCRx`))
  (for _array_element (`self.Tubes`)
    (`PrimitiveComponent.SetMaterial` _array_element 0 "/Game/StarterContent/Materials/M_Glass.M_Glass")
    (add `OscReceiverComponent.OnOscReceived` (`self.OscReceiver`) (delegate `OSCRx2`))
    (add `OscReceiverComponent.OnOscReceived` (`self.OscReceiver`) (delegate `OSCRx3`))
    (add `OscReceiverComponent.OnOscReceived` (`self.OscReceiver`) (delegate `OSCRx4`))
    (add `OscReceiverComponent.OnOscReceived` (`self.OscReceiver`) (delegate `OSCRx5`))
    (add `OscReceiverComponent.OnOscReceived` (`self.OscReceiver`) (delegate `OSCRx6`))
    (add `OscReceiverComponent.OnOscReceived` (`self.OscReceiver`) (delegate `OSCRx7`))
    (add `OscReceiverComponent.OnOscReceived` (`self.OscReceiver`) (delegate `OSCRx8`))
    (add `OscReceiverComponent.OnOscReceived` (`self.OscReceiver`) (delegate `OSCRx9`))
    (add `OscReceiverComponent.OnOscReceived` (`self.OscReceiver`) (delegate `OSCRx10`))
    (add `OscReceiverComponent.OnOscReceived` (`self.OscReceiver`) (delegate `OSCRx11`))
    (add `OscReceiverComponent.OnOscReceived` (`self.OscReceiver`) (delegate `OSCRx12`))
    (add `OscReceiverComponent.OnOscReceived` (`self.OscReceiver`) (delegate `OSCFx13`))
    (add `OscReceiverComponent.OnOscReceived` (`self.OscReceiver`) (delegate `OSCFx14`))))

(event `OSCRx`
  (params (Address :type "Name (by ref)") (Data :type "Array of OscDataElemStruct Structure (by ref)") (SenderIp :type String))
  (bind _returnvalue (`self.Check Signal` Address (`self.Leads_G2`)))
  (if _returnvalue
    (`self.LightFrontHorizontal`)))

(event `OSCRx2`
  (params (Address :type "Name (by ref)") (Data :type "Array of OscDataElemStruct Structure (by ref)") (SenderIp :type String))
  (bind _returnvalue (`self.Check Signal` Address (`self.Leads_E2`)))
  (if _returnvalue
    (`self.LightFrontCross`)))

(event `InputAction|LightAll`
  (params (Key :type "Key Structure"))
  (:`Pressed`
    (`self.LightAll` (`self.On`)))
  (:`Released`
    (`self.LightAll` (`self.Off`))))

(event `OSCRx3`
  (params (Address :type "Name (by ref)") (Data :type "Array of OscDataElemStruct Structure (by ref)") (SenderIp :type String))
  (bind _returnvalue (`self.Check Signal` Address (`self.Leads_D2`)))
  (if _returnvalue
    (`self.Light Front Frame`)))

(event `OSCRx4`
  (params (Address :type "Name (by ref)") (Data :type "Array of OscDataElemStruct Structure (by ref)") (SenderIp :type String))
  (bind _returnvalue (`self.Check Signal` Address (`self.Leads_G#1`)))
  (if _returnvalue
    (`self.LightBackHorizontal`)))

(event `OSCRx5`
  (params (Address :type "Name (by ref)") (Data :type "Array of OscDataElemStruct Structure (by ref)") (SenderIp :type String))
  (bind _returnvalue (`self.Check Signal` Address (`self.Kick_C1`)))
  (if _returnvalue
    (`self.Light Back Frame` false)))

(event `OSCRx6`
  (params (Address :type "Name (by ref)") (Data :type "Array of OscDataElemStruct Structure (by ref)") (SenderIp :type String))
  (bind _returnvalue (`self.Check Signal` Address (`self.Snare_D1`)))
  (if _returnvalue
    (`self.Light Front Frame`)))

(event `OSCRx7`
  (params (Address :type "Name (by ref)") (Data :type "Array of OscDataElemStruct Structure (by ref)") (SenderIp :type String))
  (bind _returnvalue (`self.Check Signal` Address (`self.Snare_E1`)))
  (if _returnvalue
    (`self.LightBackCross`)))

(event `OSCRx8`
  (params (Address :type "Name (by ref)") (Data :type "Array of OscDataElemStruct Structure (by ref)") (SenderIp :type String))
  (bind _returnvalue (`self.Check Signal` Address (`self.Clap_F2`)))
  (if _returnvalue
    (`self.Light Diagonals`)))

(event `OSCRx9`
  (params (Address :type "Name (by ref)") (Data :type "Array of OscDataElemStruct Structure (by ref)") (SenderIp :type String))
  (bind _returnvalue (`self.Check Signal` Address (`self.Vocals_C8`)))
  (if _returnvalue
    (`self.Light Back Frame` false)))

(event `OSCRx10`
  (params (Address :type "Name (by ref)") (Data :type "Array of OscDataElemStruct Structure (by ref)") (SenderIp :type String))
  (bind _returnvalue (`self.Check Signal` Address (`self.Vocals_C#8`)))
  (if _returnvalue
    (`self.Light Middle Frame`)))

(event `OSCRx11`
  (params (Address :type "Name (by ref)") (Data :type "Array of OscDataElemStruct Structure (by ref)") (SenderIp :type String))
  (bind _returnvalue (`self.Check Signal` Address (`self.Vocals_D8`)))
  (if _returnvalue
    (`self.Light Front Frame`)))

(event `OSCRx12`
  (params (Address :type "Name (by ref)") (Data :type "Array of OscDataElemStruct Structure (by ref)") (SenderIp :type String))
  (bind _returnvalue (`self.Check Signal` Address (`self.Clap_D#2`)))
  (if _returnvalue
    (`self.Light Middle Frame`)))

(event `OSCFx13`
  (params (Address :type "Name (by ref)") (Data :type "Array of OscDataElemStruct Structure (by ref)") (SenderIp :type String))
  (bind _returnvalue (`self.Check Signal` Address (`self.Shaker_E3`)))
  (if _returnvalue
    (`self.Light Back Cross PArt 1`)))

(event `OSCFx14`
  (params (Address :type "Name (by ref)") (Data :type "Array of OscDataElemStruct Structure (by ref)") (SenderIp :type String))
  (bind _returnvalue (`self.Check Signal` Address (`self.Shaker_F#3`)))
  (if _returnvalue
    (`self.Light Back Cross Part 2`)))

(fn `Check Signal`
  (params (SignalFrom :type Name) (TriggerNote :type String))
  (returns (ReturnValue :type Boolean))
  (return (`KismetStringLibrary.EqualEqual_StrStr` (`KismetTextLibrary.Conv_TextToString` (`|FormatText` (`KismetTextLibrary.Conv_NameToText` SignalFrom))) TriggerNote)))

(fn `Light Back Cross PArt 1`
  (if (`self.BackCrossPart1Lit`)
    (set `self.BackCrossPart1Lit` false)
    (`PrimitiveComponent.SetMaterial` (`|GetArrayItem` (`self.Tubes`) 20) 0 (`self.Off`))
    (else
      (set `self.BackCrossPart1Lit` true)
      (`PrimitiveComponent.SetMaterial` (`|GetArrayItem` (`self.Tubes`) 20) 0 (`self.On`)))))

(fn `Light Back Cross Part 2`
  (if (`self.BackCrossPart2Lit`)
    (set `self.BackCrossPart2Lit` false)
    (`PrimitiveComponent.SetMaterial` (`|GetArrayItem` (`self.Tubes`) 9) 0 (`self.Off`))
    (else
      (set `self.BackCrossPart2Lit` true)
      (`PrimitiveComponent.SetMaterial` (`|GetArrayItem` (`self.Tubes`) 9) 0 (`self.On`)))))

(fn `Light Back Frame`
  (params (Condition :type Boolean))
  (if (`self.BackFrameLit`)
    (set `self.BackFrameLit` false)
    (`self.LightFrame` (`self.Off`) 12 17 1 6)
    (else
      (set `self.BackFrameLit` true)
      (`self.LightFrame` (`self.On`) 12 17 1 6))))

(fn `Light Diagonals`
  (if (`self.DiagonalsLit`)
    (set `self.DiagonalsLit` false)
    (`self.LightFrame` (`self.Off`) 13 3 2 14)
    (else
      (set `self.DiagonalsLit` true)
      (`self.LightFrame` (`self.On`) 13 3 2 14))))

(fn `Light Front Frame`
  (if (`self.FrontFrameLit`)
    (set `self.FrontFrameLit` false)
    (`self.LightFrame` (`self.Off`) 11 8 0 21)
    (else
      (set `self.FrontFrameLit` true)
      (`self.LightFrame` (`self.On`) 11 8 0 21))))

(fn `Light Middle Frame`
  (if (`self.MiddleFrameLit`)
    (set `self.MiddleFrameLit` false)
    (`self.LightFrame` (`self.Off`) 15 7 4 22)
    (else
      (set `self.MiddleFrameLit` true)
      (`self.LightFrame` (`self.On`) 15 7 4 22))))

(fn `LightAll`
  (params (`on/off` :type "MaterialInterface Object Reference"))
  (`PrimitiveComponent.SetMaterial` (`self.Tubes`) 0 `on/off`))

(fn `LightBackCross`
  (if (`self.BackCrossLit`)
    (set `self.BackCrossLit` false)
    (`self.LightCross` (`self.Off`) 20 9)
    (else
      (set `self.BackCrossLit` true)
      (`self.LightCross` (`self.On`) 20 9))))

(fn `LightBackHorizontal`
  (if (`self.BackHorizontalLit`)
    (set `self.BackHorizontalLit` false)
    (`self.LightHorizontal` (`self.Off`) 12 9 1)
    (else
      (set `self.BackHorizontalLit` true)
      (`self.LightHorizontal` (`self.On`) 12 9 1))))

(fn `LightCross`
  (params (`on/off` :type "MaterialInterface Object Reference") (Tube1 :type Integer) (Tube2 :type Integer))
  (bind _tubes (`self.Tubes`))
  (`PrimitiveComponent.SetMaterial` (`|GetArrayItem` _tubes Tube1) 0 `on/off`)
  (`PrimitiveComponent.SetMaterial` (`|GetArrayItem` _tubes Tube2) 0 `on/off`))

(fn `LightFrame`
  (params (`on/off` :type "MaterialInterface Object Reference") (Tube1 :type Integer) (Tube2 :type Integer) (Tube3 :type Integer) (Tube4 :type Integer))
  (bind _tubes (`self.Tubes`))
  (`PrimitiveComponent.SetMaterial` (`|GetArrayItem` _tubes Tube1) 0 `on/off`)
  (`PrimitiveComponent.SetMaterial` (`|GetArrayItem` _tubes Tube2) 0 `on/off`)
  (`PrimitiveComponent.SetMaterial` (`|GetArrayItem` _tubes Tube3) 0 `on/off`)
  (`PrimitiveComponent.SetMaterial` (`|GetArrayItem` _tubes Tube4) 0 `on/off`))

(fn `LightFrontCross`
  (if (`self.FrontCrossLit`)
    (set `self.FrontCrossLit` false)
    (`self.LightCross` (`self.Off`) 18 23)
    (else
      (set `self.FrontCrossLit` true)
      (`self.LightCross` (`self.On`) 18 23))))

(fn `LightFrontHorizontal`
  (if (`self.FrontHorizontalLit`)
    (set `self.FrontHorizontalLit` false)
    (`self.LightHorizontal` (`self.Off`) 11 23)
    (else
      (set `self.FrontHorizontalLit` true)
      (`self.LightHorizontal` (`self.On`) 11 23))))

(fn `LightHorizontal`
  (params (`on/off` :type "MaterialInterface Object Reference") (Tube1 :type Integer) (Tube2 :type Integer) (Tube3 :type Integer))
  (bind _tubes (`self.Tubes`))
  (`PrimitiveComponent.SetMaterial` (`|GetArrayItem` _tubes Tube1) 0 `on/off`)
  (`PrimitiveComponent.SetMaterial` (`|GetArrayItem` _tubes Tube2) 0 `on/off`)
  (`PrimitiveComponent.SetMaterial` (`|GetArrayItem` _tubes Tube3) 0 `on/off`))

(fn `UserConstructionScript`)